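; BP_turretAuto is a player turret Blueprint that provides a hitscan shot with an impact effect.
; Its function line traces on Visibility from a supplied start point toward a point ShootDistance along the player camera's forward vector, with debug drawing.
; A hit spawns the world bullet-hit particle system, then casts the actor to BP_targetPrototype without acting on it.
; It returns true on a miss or a successful cast.
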(fn LineTraceandParticleSpawning
  (params (startpoint :type Vector))
  (bind _returnvalue (Game|GetPlayerCameraManager 0))
  (bind (_outhit _returnvalue_2) (Collision|LineTraceByChannel startpoint (+ (Transformation|GetActorLocation _returnvalue) (* (Transformation|GetActorForwardVector _returnvalue) (Variables|Default|GetShootDistance))) "TraceTypeQuery1" false 0 "ForDuration" true "(R=1.000000,G=0.000000,B=0.000000,A=1.000000)" "(R=0.000000,G=1.000000,B=0.000000,A=1.000000)" 2.0))
  (if _returnvalue_2
    (Niagara|SpawnSystematLocation "/Game/Effects/Particles/P_bulletHitWorld.P_bulletHitWorld" (.Location (Collision|BreakHitResult _outhit)))
    (Utilities|Casting|CastToBP_targetPrototype (.HitActor (Collision|BreakHitResult _outhit)))
    (return true)
    (else
      (return true))))